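; Gameplay player controller that sets up the local player's settings, HUD, sound mix and input, and opens the pause menu on Escape.
; After a short delay on BeginPlay, it loads player info from a save slot and passes it to PassCharacterInfoToServer, which stores it.
; Chat messages fan out through the GameplayGM controller list to each controller's UpdateChat, which updates its chat widget.
; The variable and widget initialisation functions are empty stubs.
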(event `self.ReceiveBeginPlay`
  ;[1 1 1] BeginPlay
  (`KismetSystemLibrary.Delay` 0.2)
  (`self.UpdatePlayer`)
  (`self.GameWidget`)
  (`GameplayStatics.SetBaseSoundMix` "/Game/AdvancedMenu/Sounds/SM_GameSoundMix.SM_GameSoundMix")
  (`WidgetBlueprintLibrary.SetInputMode_GameOnly` self))

(event `GameWidget`
  ;[1 1 1] CreteGame widget
  (bind _ascharacter (cast `Character` (`self.K2_GetPawn`)))
  (bind _returnvalue (`|CreateWidget` "/Game/AdvancedMenu/GUI/Widgets/AllLevels/WB_GameWidget.WB_GameWidget_C" null _ascharacter))
  (`UserWidget.AddToViewport` _returnvalue 0))

(event `UpdatePlayer`
  ;[1 1 1] Loads Player Info andPass to Player Controller
  (if (`self.IsLocalController`)
    (`WidgetLayoutLibrary.RemoveAllWidgets`)
    (`self.LoadGame`)
    (`self.PassCharacterInfoToServer` (`self.Player Settings`))
    ;[1 1 1] Initialize
    (`self.InitializePlayer'sVariables`)
    (`self.InitializeWidgets`)))

(event `PassCharacterInfoToServer`
  (params (`Player Settings Info` :type "/Game/AdvancedMenu/Blueprints/Multiplayer/S_PlayerInfo Structure"))
  ;[1 1 1] Passes Player Info | Respawns Player with selected character | Call setup chat window
  (set `self.Player Settings` `Player Settings Info`))

(event `GetChatMessage`
  (params (TextToSend :type Text))
  ;[1 1 1] Calls Update Chat on the client
  (set `self.SenderText` TextToSend)
  (set `self.SenderName` (`.MyPlayername_10_22484EE74A4FEB58048096BF80ADD17E` (break `/Game/AdvancedMenu/Blueprints/Multiplayer/S_PlayerInfo` (`self.Player Settings`))))
  (bind _asgameplay_gm (cast `/Game/AdvancedMenu/Blueprints/Gameplay/GameplayGM` (`GameplayStatics.GetGameMode`)))
  (for _array_element (`/Game/AdvancedMenu/Blueprints/Gameplay/GameplayGM.AllPlayerControllers` _asgameplay_gm)
    (bind _asgameplay_pc (cast `/Game/AdvancedMenu/Blueprints/Gameplay/GameplayPC` _array_element))
    (`self.UpdateChat` _asgameplay_pc (`self.SenderName`) (`self.SenderText`))))

(event `UpdateChat`
  (params (SenderName :type Text) (SenderText :type Text))
  ;[1 1 1] Updates Chat Window
  (`/Game/AdvancedMenu/GUI/Widgets/Multiplayer/WBP_Chat.UpdateChatWindow` (`/Game/AdvancedMenu/GUI/Widgets/AllLevels/WB_GameplayChat.WBP_ChatBox` (`self.GameplayChatWB`)) SenderName SenderText))

(event `Key|Escape`
  (params (Key :type "Key Structure"))
  (bind _returnvalue (`GameplayStatics.GetPlayerController` 0))
  ;[1 1 1] Open Pause Menu
  (:`Pressed`
    (bind _ascharacter (cast `Character` (`self.K2_GetPawn`)))
    (bind _returnvalue_2 (`|CreateWidget` "/Game/AdvancedMenu/GUI/Widgets/MainMenu/WBP_PauseMenu.WBP_PauseMenu_C" null _ascharacter))
    (`UserWidget.AddToViewport` _returnvalue_2 0)
    (set `PlayerController.bShowMouseCursor` true _returnvalue)
    (`WidgetBlueprintLibrary.SetInputMode_UIOnlyEx` _returnvalue _returnvalue_2)))

(fn `InitializePlayer'sVariables`)

(fn `InitializeWidgets`)

(fn `LoadGame`
  (bind _returnvalue (`GameplayStatics.LoadGameFromSlot` (`self.PlayerSettingsSave`)))
  (bind _assave_player_save_info (cast `/Game/AdvancedMenu/Saves/Save_PlayerSaveInfo` _returnvalue))
  (set `self.Player Settings` (`/Game/AdvancedMenu/Saves/Save_PlayerSaveInfo.S_PlayerInfo` _assave_player_save_info)))

(fn `UserConstructionScript`)