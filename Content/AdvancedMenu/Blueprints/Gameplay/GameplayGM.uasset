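; GameplayGM is the gameplay game mode in AdvancedMenu, handling player controller tracking and session teardown on logout.
; Controllers from OnSwapPlayerControllers are added to AllPlayerControllers, which BeginPlay loops over to set game-only input after calling SetBaseSoundMix.
; On logout, it calls DestroySession for the exiting controller if it is a GameplayPC, passing GameInstanceinfo as world context.
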(event `self.K2_OnSwapPlayerControllers`
  (params (OldPC :type "PlayerController Object Reference") (NewPC :type "PlayerController Object Reference"))
  ;[1 1 1] Track new Player Controllers
  (`KismetArrayLibrary.Array_Add` (`self.AllPlayerControllers`) NewPC))

(event `self.K2_OnLogout`
  (params (ExitingController :type "Controller Object Reference"))
  ;[1 1 1] Event on Logout | Destroysession for that PC
  (bind _asgameplay_pc (cast `/Game/AdvancedMenu/Blueprints/Gameplay/GameplayPC` ExitingController))
  (`DestroySessionCallbackProxy.DestroySession` (cast `/Game/AdvancedMenu/Blueprints/Other/GameInstanceinfo` (`GameplayStatics.GetGameInstance`) :!pure true) _asgameplay_pc))

(event `self.ReceiveBeginPlay`
  (`GameplayStatics.SetBaseSoundMix` null)
  (for _array_element (`self.AllPlayerControllers`)
    (`WidgetBlueprintLibrary.SetInputMode_GameOnly` _array_element)))

(fn `UserConstructionScript`)