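; BP_Points is a points pickup made of randomly scattered meshes that bob up and down.
; The construction script spawns SpheresCount collisionless meshes with random offset, rotation and scale, then sizes the capsule from count and padding.
; A ping-pong timeline moves each mesh along Z, reshuffling directions every cycle.
; Capsule overlap passes SpheresCount to the overlapping actor's AC_PointsSystem and destroys the pickup.
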(event `self.ReceiveBeginPlay`
  ;[1 1 1] Fill Arrays and start animation
  (`self.FillRandomInt`)
  (`self.PlayAnimation`))

(event `PlayAnimation`
  ;[1 1 1] AnimationLogic
  (`KismetArrayLibrary.Array_Shuffle` (`self.RandomIntAray`))
  (bind (_direction _value) (`Timeline|PlayMeshAnimation` :!via `PlayFromStart` :!label _label)
    (:`Update`
      (for (_array_element _array_index) (`self.Meshes`)
        (`SceneComponent.K2_SetRelativeLocation` _array_element (`self.MakeNewAnimationTransform` _array_index _value _array_element) false false)))
    (:`Finished`
      (switch `ETimelineDirection` _direction
        (:`Forward`
          (`self.ReverseAnimation`))
        (:`Backward`
          (`self.PlayAnimation`))))))

(event `ReverseAnimation`
  ;[1 1 1] AnimationLogic
  (goto _label :!via `Reverse`))

(event `self.Capsule.OnComponentBeginOverlap`
  (params (OverlappedComponent :type "PrimitiveComponent Object Reference") (OtherActor :type "Actor Object Reference") (OtherComp :type "PrimitiveComponent Object Reference") (OtherBodyIndex :type Integer) (bFromSweep :type Boolean) (SweepResult :type "HitResult Structure (by ref)"))
  ;[1 1 1] Give Player Points
  (`/Game/AdvancedMenu/Blueprints/AC_PointsSystem.AddPoints` (`self.GetComponentByClass` OtherActor "/Game/AdvancedMenu/Blueprints/AC_PointsSystem.AC_PointsSystem_C") (`self.SpheresCount`) self)
  (`self.K2_DestroyActor`))

(fn `FillRandomInt`
  (for _array_element (`self.Meshes`)
    (`KismetArrayLibrary.Array_Add` (`self.RandomIntAray`) (select `bool` (`KismetMathLibrary.RandomBoolWithWeight` 0.5) :`false` -1 :`true` 1))
    (bind (_relativelocation_x _relativelocation_y _relativelocation_z) (`KismetMathLibrary.BreakVector` (`SceneComponent.RelativeLocation` _array_element)))
    (`KismetArrayLibrary.Array_Add` (`self.RememberLocationsZ`) _relativelocation_z)))

(fn `MakeLocation`
  (params (Index :type Integer))
  (returns (Location :type "Vector Structure"))
  (bind _returnvalue (`KismetMathLibrary.Conv_IntToDouble` (* Index (`self.RandomPadding`))))
  (return (`KismetMathLibrary.MakeVector` (`self.PlusOrMinus` 0.0 (+ _returnvalue 0.0)) (`self.PlusOrMinus` 0.0 (+ _returnvalue 0.0)) (+ 0.0 (`KismetMathLibrary.RandomFloatInRange` (`self.MinZ`) (`self.MaxZ`))))))

(fn `MakeNewAnimationTransform`
  (params (Index :type Integer) (Value :type "Float (double-precision)") (Reference :type "SceneComponent Object Reference"))
  (returns (Location :type "Vector Structure"))
  (bind (_relativelocation_x _relativelocation_y) (`KismetMathLibrary.BreakVector` (`SceneComponent.RelativeLocation` Reference)))
  (return (`KismetMathLibrary.MakeVector` _relativelocation_x _relativelocation_y (+ (`|GetArrayItem` (`self.RememberLocationsZ`) Index) (* Value (`KismetMathLibrary.Conv_IntToDouble` (`|GetArrayItem` (`self.RandomIntAray`) Index)))))))

(fn `MakeRotation`
  (returns (Rotation :type "Rotator Structure"))
  (bind (_returnvalue_roll _returnvalue_pitch _returnvalue_yaw) (`KismetMathLibrary.BreakRotator` (`self.K2_GetActorRotation`)))
  (bind (_randomaddrotation_roll _randomaddrotation_pitch _randomaddrotation_yaw) (`KismetMathLibrary.BreakRotator` (`self.RandomAddRotation`)))
  (return (`KismetMathLibrary.MakeRotator` (`self.PlusOrMinus` _returnvalue_roll _randomaddrotation_roll) (`self.PlusOrMinus` _returnvalue_pitch _randomaddrotation_pitch) (`self.PlusOrMinus` _returnvalue_yaw _randomaddrotation_yaw))))

(fn `MakeSize`
  (returns (ReturnValue :type "Vector Structure"))
  (bind _returnvalue (`KismetMathLibrary.RandomFloatInRange` (`self.MinSize`) (`self.MaxSize`)))
  (return (`KismetMathLibrary.MakeVector` _returnvalue _returnvalue _returnvalue)))

(fn `PlusOrMinus`
  (params (A :type "Float (double-precision)") (B :type "Float (double-precision)"))
  (returns (ReturnValue :type "Float (double-precision)"))
  (return (select `bool` (`KismetMathLibrary.RandomBoolWithWeight` 0.5) :`false` (`KismetMathLibrary.Conv_IntToDouble` (+ (`KismetMathLibrary.FTrunc` A) (`KismetMathLibrary.FTrunc` B))) :`true` (`KismetMathLibrary.Conv_IntToDouble` (- (`KismetMathLibrary.FTrunc` A) (`KismetMathLibrary.FTrunc` B))))))

(fn `RandomPadding`
  (returns (ReturnValue :type Integer))
  (bind _meshespadding (`self.MeshesPadding`))
  (return (`KismetMathLibrary.RandomIntegerInRange` (- _meshespadding (/ _meshespadding 2)) (+ _meshespadding (/ _meshespadding 2)))))

(fn `SetNewCapsuleSize`
  (params (LastIndex :type Integer))
  (bind _capsule (`self.Capsule`))
  (bind _returnvalue (`KismetMathLibrary.Conv_IntToDouble` (* (+ LastIndex 1) (`self.MeshesPadding`))))
  (`CapsuleComponent.SetCapsuleRadius` _capsule _returnvalue true)
  (`CapsuleComponent.SetCapsuleHalfHeight` _capsule (* _returnvalue 2.0) true))

(fn `UserConstructionScript`
  (for _index (range (`self.SpheresCount`))
    ;[1 1 1] Create Mesh With New Location
    (bind _returnvalue (`AddComponent|NODE_AddStaticMeshComponent-0` :`RelativeTransform` (`KismetMathLibrary.MakeTransform` (`self.MakeLocation` _index) (`self.MakeRotation`) (`self.MakeSize`))))
    (`KismetArrayLibrary.Array_Add` (`self.Meshes`) _returnvalue)
    ;[1 1 1] Set Mesh And Material
    (`StaticMeshComponent.SetStaticMesh` _returnvalue (`self.Mesh`))
    (`PrimitiveComponent.SetMaterial` _returnvalue 0 (`self.Material`))
    (`PrimitiveComponent.SetCollisionEnabled` _returnvalue "NoCollision"))
  (`self.SetNewCapsuleSize` _index))