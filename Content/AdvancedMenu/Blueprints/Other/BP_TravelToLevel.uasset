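; BP_TravelToLevel is a level-travel trigger: a Character overlapping its sphere starts travel to the LevelIndex level.
; On overlap it checks the GameInstance's SoloPlay flag, calling Teleport-Solo directly or Teleport-Server, which calls Teleport-All.
; Both paths share logic that loads the current save slot and passes its information to the GameInstance's TravelToLevel.
; The construction script sizes the sphere from SphereRadius.
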(event `self.ReceiveBeginPlay`
  ;[1 1 1] Begin Play
  (bind _asgame_instanceinfo (cast `/Game/AdvancedMenu/Blueprints/Other/GameInstanceinfo` (`GameplayStatics.GetGameInstance`)))
  (set `self.GameInstance` _asgame_instanceinfo))

(event `Teleport -Server`
  ;[1 1 1] Begin Play
  (`self.Teleport -All`))

(event `Teleport -Solo`
  (bind _gameinstance (`self.GameInstance`))
  ;[1 1 1] Travel to level on overlap
  (bind (_exist _information) (`/Game/AdvancedMenu/Blueprints/Other/GameInstanceinfo.LoadGame` _gameinstance (`/Game/AdvancedMenu/Blueprints/Other/GameInstanceinfo.SlotIndex` _gameinstance) :!label _label))
  (`/Game/AdvancedMenu/Blueprints/Other/GameInstanceinfo.TravelToLevel` (`self.GameInstance`) (`self.LevelIndex`) true _information true))

(event `self.Sphere.OnComponentBeginOverlap`
  (params (OverlappedComponent :type "PrimitiveComponent Object Reference") (OtherActor :type "Actor Object Reference") (OtherComp :type "PrimitiveComponent Object Reference") (OtherBodyIndex :type Integer) (bFromSweep :type Boolean) (SweepResult :type "HitResult Structure (by ref)"))
  ;[1 1 1] Travel to level on overlap
  (cast `Character` OtherActor)
  (if (`/Game/AdvancedMenu/Blueprints/Other/GameInstanceinfo.SoloPlay?` (`self.GameInstance`))
    (`self.Teleport -Solo`)
    (else
      (`self.Teleport -Server`))))

(event `Teleport -All`
  ;[1 1 1] Travel to level on overlap
  (goto _label))

(fn `UserConstructionScript`
  (`SphereComponent.SetSphereRadius` (`self.Sphere`) (`self.SphereRadius`) true))