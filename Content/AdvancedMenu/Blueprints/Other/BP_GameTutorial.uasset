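; BP_GameTutorial is a trigger actor that shows a tutorial prompt when a Character enters its box.
; The overlap sets that character as owner, then calls PlayTutorial through a server-named event.
; PlayTutorial loads the saved properties and, if tutorials are enabled, creates WB_Tutorial for the character's controller with the configured input action and text.
; The actor then destroys itself, even with tutorials disabled, unless the save fails to load.
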(event `PlayTutorial`
  (params (Target :type "Pawn Object Reference"))
  ;[1 1 1] PlayDialogue
  (bind _returnvalue (`GameplayStatics.LoadGameFromSlot` (`self.Property`)))
  (bind _assave_properties (cast `/Game/AdvancedMenu/Saves/Save_Properties` _returnvalue))
  (if (`/Game/AdvancedMenu/Saves/Save_Properties.STutorial` _assave_properties)
    (bind _returnvalue_2 (`|CreateWidget` "/Game/AdvancedMenu/GUI/Widgets/AllLevels/WB_Tutorial.WB_Tutorial_C" (cast `PlayerController` (`Pawn.GetController` Target) :!pure true) (`self.AxisOrActionName`) (`self.TutorialText`)))
    (`UserWidget.AddToViewport` _returnvalue_2 0))
  (`self.K2_DestroyActor`))

(event `self.Box.OnComponentBeginOverlap`
  (params (OverlappedComponent :type "PrimitiveComponent Object Reference") (OtherActor :type "Actor Object Reference") (OtherComp :type "PrimitiveComponent Object Reference") (OtherBodyIndex :type Integer) (bFromSweep :type Boolean) (SweepResult :type "HitResult Structure (by ref)"))
  (bind _ascharacter (cast `Character` OtherActor))
  (`self.SetOwner` _ascharacter)
  (`self.PlayTutorial -Server` _ascharacter))

(event `PlayTutorial -Server`
  (params (Target :type "Pawn Object Reference"))
  (`self.PlayTutorial` Target))

(fn `UserConstructionScript`)