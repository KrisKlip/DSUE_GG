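; Preview drone for calibration that visualizes thrust, yaw, pitch and roll input on its mesh.
; UpdateDrone routes each axis value to a handler that maps it to mesh height for thrust or to a stored rotator for the other axes.
; Tick combines roll and pitch, then applies yaw around the tilted up vector to set the mesh's relative rotation.
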(event `self.ReceiveBeginPlay`
  (set `self.StartingLocation` (`self.K2_GetActorLocation`)))

(event `self.ReceiveTick`
  (params (DeltaSeconds :type "Float (single-precision)"))
  (bind (_yawrotator_roll _yawrotator_pitch _yawrotator_yaw) (`KismetMathLibrary.BreakRotator` (`self.yawRotator`)))
  (bind _returnvalue (`KismetMathLibrary.ComposeRotators` (`self.RollRotator`) (`self.PitchRotator`)))
  (`SceneComponent.K2_SetRelativeRotation` (`self.DroneMesh`) (`KismetMathLibrary.ComposeRotators` _returnvalue (`KismetMathLibrary.RotatorFromAxisAndAngle` (`KismetMathLibrary.GetUpVector` _returnvalue) _yawrotator_yaw)) false false))

(event `UpdateThrottle`
  (params (InValue :type "Float (double-precision)"))
  (`SceneComponent.K2_SetRelativeLocation` (`self.DroneMesh`) (`KismetMathLibrary.MakeVector` 0.0 0.0 (`KismetMathLibrary.MapRangeClamped` InValue 0.0 1.0 0.0 100.0)) false false))

(event `UpdateRoll`
  (params (InValue :type "Float (double-precision)"))
  (set `self.RollRotator` (`KismetMathLibrary.MakeRotator` (`KismetMathLibrary.MapRangeClamped` (`KismetMathLibrary.Abs` InValue) 0.0 1.0 -45.0 45.0))))

(event `UpdatePitch`
  (params (InValue :type "Float (double-precision)"))
  (bind _output_get (set `self.PitchRotator` (`KismetMathLibrary.MakeRotator` 0.0 (`KismetMathLibrary.MapRangeClamped` (`KismetMathLibrary.Abs` InValue) 0.0 1.0 45.0 -45.0)))))

(event `UpdateYaw`
  (params (InValue :type "Float (double-precision)"))
  (set `self.yawRotator` (`KismetMathLibrary.MakeRotator` 0.0 0.0 (`KismetMathLibrary.MapRangeClamped` (`KismetMathLibrary.Abs` InValue) 0.0 1.0 -45.0 45.0))))

(event `UpdateDrone`
  (params (Axis :type String) (InValue :type "Float (double-precision)"))
  (switch `string` Axis
    (:`Thrust`
      (`self.UpdateThrottle` InValue))
    (:`Yaw`
      (`self.UpdateYaw` InValue))
    (:`Pitch`
      (`self.UpdatePitch` InValue))
    (:`Roll`
      (`self.UpdateRoll` InValue))))

(fn `UserConstructionScript`)