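; MiniFortress is a turret-style actor in the lock-on system that, when enabled, periodically launches homing MiniMissiles at its Target.
; On BeginPlay it tags itself with its team and type and applies its material.
; A looping timer spawns each missile at the next numbered static mesh socket, cycling through them, and starts homing immediately.
; A delayed for-loop macro is defined but unused in the shown graphs.
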(event `self.ReceiveBeginPlay`
  (set `self.Tags` (`|MakeArray` (`self.Team`) (`KismetStringLibrary.Conv_StringToName` (`|GetEnumeratorNameAsString` (`self.Type`)))))
  (`PrimitiveComponent.SetMaterial` (`self.StaticMesh`) 0 (`self.Material`))
  (if (`self.Enable`)
    (`KismetSystemLibrary.K2_SetTimerDelegate` (delegate `SingleFire`) 3.0 true)))

(event `SingleFire`
  (bind _returnvalue (`KismetStringLibrary.Conv_StringToName` (`KismetStringLibrary.Conv_IntToString` (`self.Socket`))))
  (bind _returnvalue_2 (`|SpawnActorFromClass` "/Game/AdvancedLockonSystem/Blueprints/Actor/Projectile/MiniMissile.MiniMissile_C" (`KismetMathLibrary.MakeTransform` (`SceneComponent.GetSocketLocation` (`self.StaticMesh`) _returnvalue) (`SceneComponent.GetSocketRotation` (`self.StaticMesh`) _returnvalue)) "AdjustIfPossibleButAlwaysSpawn" "OverrideRootScale" self null))
  (`/Game/AdvancedLockonSystem/Blueprints/Actor/Projectile/MiniMissile.Homing` _returnvalue_2 (`self.Target`) 0.0)
  (bind _output_get (set `self.Socket` (+ (`self.Socket`) 1)))
  (if (> _output_get 20)
    (set `self.Socket` 1)))

(fn `UserConstructionScript`)