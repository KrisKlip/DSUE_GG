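; Cluster-style homing missile for the lock-on system that splits into child missiles to attack multiple targets.
; Homing steers the projectile movement toward a VectorTarget actor, while a Radar sphere, resized to the detonation distance shortly after spawn, watches for listed targets.
; Overlapping one spawns a child homing missile per valid target, then destroys the parent and VectorTarget.
; Hits, incoming damage or an empty target list (checked by timer) also explode both, with only hits applying damage.
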(event `self.ReceiveBeginPlay`
  ;[1 1 1] Set actor tags
  (set `self.Tags` (`|MakeArray` (`|GetArrayItem` (`Actor.Tags` (`self.GetOwner`))) (`KismetStringLibrary.Conv_StringToName` (`|GetEnumeratorNameAsString` (`self.Type`)))))
  (`KismetSystemLibrary.K2_SetTimerDelegate` (delegate `Target Check`) 1.0 true)
  (`KismetSystemLibrary.Delay` 0.5)
  (`SphereComponent.SetSphereRadius` (`self.Radar`) (`self.DetonateDistance`) true))

(event `Target Check`
  (bind _returnvalue (`self.K2_GetActorLocation`))
  ;[1 1 1] If the target is not valid, destroy self.
  (if (not (`KismetArrayLibrary.Array_IsValidIndex` (stale `Homing` `Homin Target Array`)))
    (`KismetSystemLibrary.Delay` 3.0)
    (`GameplayStatics.SpawnEmitterAtLocation` "/Game/AdvancedLockonSystem/ExampleContent/Effects/ParticleSystems/Weapons/RocketLauncher/Impact/P_Launcher_IH.P_Launcher_IH" _returnvalue (struct) (5.0 5.0 5.0))
    (`GameplayStatics.PlaySoundAtLocation` "/Game/AdvancedLockonSystem/ExampleContent/Sounds/Cue/GrenadeLauncher_Explosion_Cue.GrenadeLauncher_Explosion_Cue" _returnvalue)
    (`self.K2_DestroyActor` (`self.VectorTarget`))
    (`self.K2_DestroyActor`)))

(event `Homing`
  (params (VectorTarget :type "Actor Object Reference") (`Homin Target Array` :type "Array of Actor Object Reference"))
  (bind _projectilemovement (`self.ProjectileMovement`))
  ;[1 1 1] Set homing to the vector target.
  (`KismetSystemLibrary.PrintString` (`KismetStringLibrary.Conv_IntToString` (`KismetArrayLibrary.Array_Length` `Homin Target Array`)) true true (struct :`R` 1.0 :`B` 0.106359 :`A` 1.0))
  (set `self.VectorTarget` VectorTarget)
  (if (`KismetSystemLibrary.IsValid` VectorTarget)
    (set `ProjectileMovementComponent.bIsHomingProjectile` true _projectilemovement)
    (set `ProjectileMovementComponent.HomingAccelerationMagnitude` 5000.0 _projectilemovement)
    (set `ProjectileMovementComponent.HomingTargetComponent` (`Actor.RootComponent` (`self.VectorTarget`)) _projectilemovement)))

(event `self.Radar.OnComponentBeginOverlap`
  (params (OverlappedComponent :type "PrimitiveComponent Object Reference") (OtherActor :type "Actor Object Reference") (OtherComp :type "PrimitiveComponent Object Reference") (OtherBodyIndex :type Integer) (bFromSweep :type Boolean) (SweepResult :type "HitResult Structure (by ref)"))
  ;[1 1 1] If the vector target is detected at the detonate distance, child homing is executed.
  (if (`KismetArrayLibrary.Array_Contains` (stale `Homing` `Homin Target Array`) OtherActor)
    (`self.Child Homing`)
    (else
      (`KismetSystemLibrary.PrintString` "sdffslkdjflksjdflkjsdlkfjlskdjflksjdflsdf"))))

(event `Child Homing`
  (bind _returnvalue (`self.K2_GetActorLocation`))
  ;[1 1 1] Shoot child homing missiles to targets
  (for _array_element (stale `Homing` `Homin Target Array`)
    (if (`KismetSystemLibrary.IsValid` _array_element)
      (`KismetSystemLibrary.PrintString` (`KismetSystemLibrary.GetDisplayName` _array_element) true true (struct :`R` 1.0 :`G` 0.833552 :`A` 1.0))
      (bind _returnvalue_2 (`|SpawnActorFromClass` "/Game/AdvancedLockonSystem/Blueprints/Projectile/ChildHomingMissile.ChildHomingMissile_C" (`KismetMathLibrary.MakeTransform` (`self.K2_GetActorLocation`) (`self.K2_GetActorRotation`) (5.0 5.0 5.0)) "AdjustIfPossibleButAlwaysSpawn" "OverrideRootScale" (`self.GetOwner`) null))
      (`/Game/AdvancedLockonSystem/Blueprints/Projectile/ChildHomingMissile.Homing` _returnvalue_2 _array_element)))
  ;[1 1 1] Destroy vector target and self
  (`GameplayStatics.SpawnEmitterAtLocation` "/Game/AdvancedLockonSystem/ExampleContent/Effects/ParticleSystems/Weapons/RocketLauncher/Impact/P_Launcher_IH.P_Launcher_IH" _returnvalue (struct) (5.0 5.0 5.0))
  (`GameplayStatics.PlaySoundAtLocation` "/Game/AdvancedLockonSystem/ExampleContent/Sounds/Cue/GrenadeLauncher_Explosion_Cue.GrenadeLauncher_Explosion_Cue" _returnvalue)
  (`self.K2_DestroyActor` (`self.VectorTarget`))
  (`self.K2_DestroyActor`))

(event `self.ReceiveHit`
  (params (MyComp :type "PrimitiveComponent Object Reference") (Other :type "Actor Object Reference") (OtherComp :type "PrimitiveComponent Object Reference") (bSelfMoved :type Boolean) (HitLocation :type "Vector Structure") (HitNormal :type "Vector Structure") (NormalImpulse :type "Vector Structure") (Hit :type "HitResult Structure (by ref)"))
  (`GameplayStatics.ApplyDamage` Other 1.0)
  (`GameplayStatics.SpawnEmitterAtLocation` "/Game/AdvancedLockonSystem/ExampleContent/Effects/ParticleSystems/Weapons/RocketLauncher/Impact/P_Launcher_IH.P_Launcher_IH" HitLocation (struct) (5.0 5.0 5.0))
  (`GameplayStatics.PlaySoundAtLocation` "/Game/AdvancedLockonSystem/ExampleContent/Sounds/Cue/GrenadeLauncher_Explosion_Cue.GrenadeLauncher_Explosion_Cue" HitLocation)
  (`self.K2_DestroyActor` (`self.VectorTarget`))
  (`self.K2_DestroyActor`))

(event `self.ReceiveAnyDamage`
  (params (Damage :type "Float (single-precision)") (DamageType :type "DamageType Object Reference") (InstigatedBy :type "Controller Object Reference") (DamageCauser :type "Actor Object Reference"))
  (bind _returnvalue (`self.K2_GetActorLocation`))
  (`GameplayStatics.SpawnEmitterAtLocation` "/Game/AdvancedLockonSystem/ExampleContent/Effects/ParticleSystems/Weapons/RocketLauncher/Impact/P_Launcher_IH.P_Launcher_IH" _returnvalue (struct) (5.0 5.0 5.0))
  (`GameplayStatics.PlaySoundAtLocation` "/Game/AdvancedLockonSystem/ExampleContent/Sounds/Cue/GrenadeLauncher_Explosion_Cue.GrenadeLauncher_Explosion_Cue" _returnvalue)
  (`self.K2_DestroyActor` (`self.VectorTarget`))
  (`self.K2_DestroyActor`))

(fn `UserConstructionScript`)