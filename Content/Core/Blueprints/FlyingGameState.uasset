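; Game state that configures a match from saved options and manages split-screen players and session teardown.
; After a short delay on BeginPlay, the authority loads the GameOptions save, setting player count, game mode and local-play flag, then creates extra players for local games.
; Ending a hosted session destroys it and removes extra players through the DebugRemovePlayer console command, a noted workaround for unreliable RemovePlayer.
; PlayerJoin only flags the listen server as joined.
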(event `self.ReceiveBeginPlay`
  (bind _printdebugonscreen (`self.PrintDebugOnScreen`))
  ;[1 1 1] Load GameOptions
  (`KismetSystemLibrary.Delay` 1.0)
  (`/Engine/EditorBlueprintResources/ActorMacros.Switch Has Authority`
    (:`Authority`
      (bind _returnvalue (`GameplayStatics.LoadGameFromSlot` "GameOptions"))
      (bind _asbp_save_game (cast `/Game/Cardinal/MainMenu/Blueprints/Saves/BP_SaveGame` _returnvalue))
      (bind _output_get (set `self.BP_SaveGame` _asbp_save_game))
      (set `self.NumberOfPlayersSetForMatch` (`/Game/Cardinal/MainMenu/Blueprints/Saves/BP_SaveGame.NumberPlayers` _output_get))
      (bind _enumvalue (foreach `/Game/Cardinal/MainMenu/Blueprints/Enum_GameModes`)
        (:`LoopBody`
          (if (== (`self.GameModeCount`) (`/Game/Cardinal/MainMenu/Blueprints/Saves/BP_SaveGame.GameMode` _output_get))
            (set `self.GameMode` _enumvalue))
          (`/Engine/EditorBlueprintResources/StandardMacros.IncrementInt` (`self.GameModeCount`)))
        (:`then`
          (`KismetSystemLibrary.PrintString` (`|GetEnumeratorNameAsString` (`self.GameMode`)))
          (bind _output_get_2 (set `self.IsLocalPlay?` (`/Game/Cardinal/MainMenu/Blueprints/Saves/BP_SaveGame.IsLocalPlay?` (`self.BP_SaveGame`))))
          (if _output_get_2
            (`KismetSystemLibrary.PrintString` "Local Game" _printdebugonscreen _printdebugonscreen)
            (`self.Spawn Split Screen Players`)
            (else
              (`KismetSystemLibrary.PrintString` "Multiplayer Game" _printdebugonscreen _printdebugonscreen))))))))

(event `End Host Online Session`
  (bind _printdebugonscreen (`self.PrintDebugOnScreen`))
  ;[1 1 1] End Host Online Session
  (`DestroySessionCallbackProxy.DestroySession` (`GameplayStatics.GetPlayerController` 0)
    (:`then`
      (for _index (range (+ (+ (`self.NumberOfPlayersSetForMatch`) -1) 1))
        (if (> _index 0)
          (`KismetSystemLibrary.ExecuteConsoleCommand` (`KismetStringLibrary.Concat_StrStr` "DebugRemovePlayer " (`KismetStringLibrary.Conv_IntToString` _index)) (`GameplayStatics.GetPlayerController` 0)))))
    (:`OnSuccess`
      (`KismetSystemLibrary.PrintString` "Server Destroy Session Success" _printdebugonscreen _printdebugonscreen))
    (:`OnFailure`
      (`KismetSystemLibrary.PrintString` "Server Destroy Session Failure" _printdebugonscreen _printdebugonscreen))))

(event `Player Join`
  ;[1 1 1] Player Join
  (set `self.IsListenServerAlreadyJoined?` true))

(event `Spawn Split Screen Players`
  ;[1 1 1] Spawn Split Screen Players
  (for _index (range (+ (+ (`self.NumberOfPlayersSetForMatch`) -1) 1))
    (if (> _index 0)
      (`GameplayStatics.CreatePlayer` _index))))

(fn `UserConstructionScript`)