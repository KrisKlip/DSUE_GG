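; Player controller for the drone game that switches between a FlyingPawn and a DrawingPawn and toggles the pause menu.
; Keys 1 and 2 possess the first actor found of each pawn class and disable input acceptance on the FlyingPawn cached at BeginPlay.
; Axis inputs cast the controlled pawn, routing gate pitch and yaw to DrawingPawn and camera FOV and angle to FlyingPawn.
; P flips the game state in BP_GameInstance.
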(event `InputAxis|GateRotateForwardBack`
  (params (AxisValue :type "Float (single-precision)"))
  (bind _asdrawing_pawn (cast `/Game/Core/Blueprints/DrawingPawn` (`self.K2_GetPawn`)))
  (`/Game/Core/Blueprints/DrawingPawn.PitchActiveGate` _asdrawing_pawn AxisValue))

(event `InputAxis|GateRotateLeftRight`
  (params (AxisValue :type "Float (single-precision)"))
  (bind _asdrawing_pawn (cast `/Game/Core/Blueprints/DrawingPawn` (`self.K2_GetPawn`)))
  (`/Game/Core/Blueprints/DrawingPawn.YawACtiveGate` _asdrawing_pawn AxisValue))

(event `Key|Two`
  (params (Key :type "Key Structure"))
  (:`Pressed`
    (bind _outactors (`GameplayStatics.GetAllActorsOfClass` "/Game/Core/Blueprints/DrawingPawn.DrawingPawn_C"))
    (`self.Possess` (`|GetArrayItem` _outactors))
    (set `/Game/Core/Blueprints/FlyingPawn.bAcceptInput` false (`self.CharacterRef`))))

(event `Key|One`
  (params (Key :type "Key Structure"))
  (:`Pressed`
    (bind _outactors (`GameplayStatics.GetAllActorsOfClass` "/Game/Core/Blueprints/FlyingPawn.FlyingPawn_C"))
    (`self.Possess` (`|GetArrayItem` _outactors))
    (set `/Game/Core/Blueprints/FlyingPawn.bAcceptInput` false (`self.CharacterRef`))))

(event `InputAxis|CameraFOV`
  (params (AxisValue :type "Float (single-precision)"))
  (bind _asflying_pawn (cast `/Game/Core/Blueprints/FlyingPawn` (`self.K2_GetPawn`)))
  (`/Game/Core/Blueprints/FlyingPawn.SetFOV` _asflying_pawn AxisValue))

(event `InputAxis|CameraAngle`
  (params (AxisValue :type "Float (single-precision)"))
  (bind _asflying_pawn (cast `/Game/Core/Blueprints/FlyingPawn` (`self.K2_GetPawn`)))
  (`/Game/Core/Blueprints/FlyingPawn.SetCameraAngle` _asflying_pawn AxisValue))

(event `Key|P` :paused true
  (params (Key :type "Key Structure"))
  ;[0 1 1 0.5] Pause Game/Access In-Game Menu
  (:`Pressed`
    (bind _asbp_game_instance (cast `/Game/PrototypeMenuSystem/Blueprints/BP_GameInstance` (`GameplayStatics.GetGameInstance`)))
    (switch `/Game/PrototypeMenuSystem/Blueprints/Enums/EGameState` (`/Game/PrototypeMenuSystem/Blueprints/BP_GameInstance.GameState` _asbp_game_instance)
      (:`NewEnumerator1`
        (`/Game/PrototypeMenuSystem/Blueprints/BP_GameInstance.SetGameState` _asbp_game_instance "NewEnumerator6"))
      (:`NewEnumerator6`
        (`/Game/PrototypeMenuSystem/Blueprints/BP_GameInstance.SetGameState` _asbp_game_instance "NewEnumerator1")))))

(event `self.ReceiveBeginPlay`
  (`|ExecutionSequence`
    (:`then_0`
      (bind _asflying_pawn (cast `/Game/Core/Blueprints/FlyingPawn` (`GameplayStatics.GetPlayerPawn` 0)))
      (set `self.CharacterRef` _asflying_pawn))))

(fn `UserConstructionScript`)