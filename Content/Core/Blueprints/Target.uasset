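; A destructible target actor that a character can lock onto, exposing a homing location and a destroyed state.
; LockonTime timestamps the start of a lock and, on later calls once the required time has passed, adds the target to the character's LockedTargets; unlocking resets the timer.
; When the Destructible component fractures, it removes the static mesh, flags itself destroyed and destroys the actor after a delay.
; Hit and lock events print debug strings.
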(event `self.Destructible.OnComponentFracture`
  (params (HitPoint :type "Vector Structure (by ref)") (HitDirection :type "Vector Structure (by ref)"))
  (`ActorComponent.K2_DestroyComponent` (`self.StaticMesh`))
  (set `self.bDestroyed` true)
  (`KismetSystemLibrary.Delay` 5.0)
  (`self.K2_DestroyActor`))

(event `self.StaticMesh.OnComponentHit`
  (params (HitComponent :type "PrimitiveComponent Object Reference") (OtherActor :type "Actor Object Reference") (OtherComp :type "PrimitiveComponent Object Reference") (NormalImpulse :type "Vector Structure") (Hit :type "HitResult Structure (by ref)"))
  (`KismetSystemLibrary.PrintString` "dESTRUCT"))

(event `/Game/Core/Blueprints/TargetInterface.LockOnTime`
  (params (isLocked :type Boolean) (CharRef :type "/Game/Core/Blueprints/FlyingPawn Object Reference"))
  (bind _returnvalue (`KismetSystemLibrary.GetGameTimeInSeconds`))
  (if isLocked
    (`KismetSystemLibrary.PrintString` "locked" false true (struct :`R` 0.270008 :`G` 1.0 :`A` 1.0))
    (if (< (`self.StartTime`) 0.0)
      (set `self.StartTime` _returnvalue)
      (elif (>= (- _returnvalue (`self.StartTime`)) (`self.RequiredLockTime`))
        (`KismetArrayLibrary.Array_AddUnique` (`/Game/Core/Blueprints/FlyingPawn.LockedTargets` CharRef) self)))
    (else
      (`KismetSystemLibrary.PrintString` "Unlocked" false true (struct :`R` 1.0 :`A` 1.0))
      (set `self.StartTime` -1.0))))

(fn `Destroyed`
  (returns (destroyed :type Boolean))
  (return (`self.bDestroyed`)))

(fn `HomingLocation`
  (returns (homingLoc :type "SceneComponent Object Reference"))
  (return (`self.HomingLoc`)))

(fn `UserConstructionScript`)