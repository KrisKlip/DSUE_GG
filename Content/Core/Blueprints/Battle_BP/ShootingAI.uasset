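; ShootingAI is a destructible turret-style enemy that fires homing missiles at the FightingPawn and can itself be locked on as a target.
; Pawn sensing turns its pivot toward the seen pawn and spawns homing projectiles, throttled by a delayed flag.
; LockonTime adds it to the caller's locked targets after a sustained lock.
; Fracturing stops firing and destroys the actor after a delay, while getters expose destroyed state and homing location.
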(event `self.Destructible.OnComponentFracture`
  (params (HitPoint :type "Vector Structure (by ref)") (HitDirection :type "Vector Structure (by ref)"))
  (set `self.bDestroyed` true)
  (`KismetSystemLibrary.Delay` 5.0)
  (`self.K2_DestroyActor`))

(event `self.StaticMesh.OnComponentHit`
  (params (HitComponent :type "PrimitiveComponent Object Reference") (OtherActor :type "Actor Object Reference") (OtherComp :type "PrimitiveComponent Object Reference") (NormalImpulse :type "Vector Structure") (Hit :type "HitResult Structure (by ref)"))
  (`KismetSystemLibrary.PrintString` "dESTRUCT"))

(event `/Game/Core/Blueprints/Battle_BP/TargetInterface.LockOnTime`
  (params (isLocked :type Boolean) (CharRef :type "/Game/Core/Blueprints/Characters/FightingPawn Object Reference"))
  (bind _returnvalue (`KismetSystemLibrary.GetGameTimeInSeconds`))
  (if isLocked
    (`KismetSystemLibrary.PrintString` "locked" false true (struct :`R` 0.270008 :`G` 1.0 :`A` 1.0))
    (if (< (`self.StartTime`) 0.0)
      (set `self.StartTime` _returnvalue)
      (elif (>= (- _returnvalue (`self.StartTime`)) (`self.RequiredLockTime`))
        (`KismetArrayLibrary.Array_AddUnique` (`/Game/Core/Blueprints/Characters/FightingPawn.LockedTargets` CharRef) self)))
    (else
      (`KismetSystemLibrary.PrintString` "Unlocked" false true (struct :`R` 1.0 :`A` 1.0))
      (set `self.StartTime` -1.0))))

(event `self.PawnSensing.OnSeePawn`
  (params (Pawn :type "Pawn Object Reference"))
  (if (not (`self.bDestroyed`))
    (bind _asfighting_pawn (cast `/Game/Core/Blueprints/Characters/FightingPawn` Pawn))
    (`|ExecutionSequence`
      (:`then_0`
        (`SceneComponent.K2_SetWorldRotation` (`self.RotationPivot`) (`KismetMathLibrary.FindLookAtRotation` (`self.K2_GetActorLocation`) (`self.K2_GetActorLocation` _asfighting_pawn)) false false)
        (`KismetSystemLibrary.PrintString` "Hello"))
      (:`then_1`
        (if (`self.SpawnProjectile`)
          (bind _returnvalue (`|SpawnActorFromClass` "/Game/Core/Blueprints/Battle_BP/HomingProjectile.HomingProjectile_C" (`SceneComponent.K2_GetComponentToWorld` (`self.SpawnProjectile Location`)) "Undefined" "OverrideRootScale" null null))
          (`/Game/Core/Blueprints/Battle_BP/HomingProjectile.HomingMissile` _returnvalue _asfighting_pawn 3000.0 10000.0)
          (`/Game/Core/Blueprints/Battle_BP/HomingProjectile.SetShooter` _returnvalue self)
          (set `self.SpawnProjectile` false)
          (`KismetSystemLibrary.Delay` 1.0)
          (set `self.SpawnProjectile` true))))))

(fn `Destroyed`
  (returns (destroyed :type Boolean))
  (return (`self.bDestroyed`)))

(fn `HomingLocation`
  (returns (homingLoc :type "SceneComponent Object Reference"))
  (return (`self.HomingLoc`)))

(fn `UserConstructionScript`)