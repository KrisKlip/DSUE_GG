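; Race manager that runs a looping gate course and reports timing and lap events to FlyingGameState.
; On BeginPlay it resets the Gates array, then keeps one gate active at a time, binding only that gate's box overlap.
; Each overlap deactivates the gate and activates the next, wrapping after the last.
; The first trigger starts the stopwatch; crossing the first gate again after a wrap counts a lap.
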(event `self.ReceiveBeginPlay`
  (`|ExecutionSequence`
    (:`then_0`
      (bind _asflying_game_state (cast `/Game/Core/Blueprints/FlyingGameState` (`GameplayStatics.GetGameState`)))
      (set `self.FlyingGameState` _asflying_game_state))
    (:`then_1`
      (for _array_element (`self.Gates`)
        (`/Game/Core/Blueprints/Racing_BP/Gate_BP.InitializeGate` _array_element)
        (`/Game/Core/Blueprints/Racing_BP/Gate_BP.SetGatePassive` _array_element))
      (`self.SetActiveGate`)
      (`self.InitializeNextGate`))))

(event `DisableLastGate`
  (bind _activegateref (`self.ActiveGateRef`))
  (`/Engine/EditorBlueprintResources/StandardMacros.IsValid` _activegateref
    (:`Is Valid`
      (clear `PrimitiveComponent.OnComponentBeginOverlap` (`/Game/Core/Blueprints/Racing_BP/Gate_BP.Box` _activegateref))
      (`/Game/Core/Blueprints/Racing_BP/Gate_BP.SetGatePassive` _activegateref))))

(event `InitializeNextGate`
  (bind _activegateref (`self.ActiveGateRef`))
  (`/Engine/EditorBlueprintResources/StandardMacros.IsValid` _activegateref
    (:`Is Valid`
      (add `PrimitiveComponent.OnComponentBeginOverlap` (`/Game/Core/Blueprints/Racing_BP/Gate_BP.Box` _activegateref) (delegate `GateTriggered`)))))

(event `GateTriggered`
  (params (OverlappedComponent :type "PrimitiveComponent Object Reference") (OtherActor :type "Actor Object Reference") (OtherComp :type "PrimitiveComponent Object Reference") (OtherBodyIndex :type Integer) (bFromSweep :type Boolean) (SweepResult :type "HitResult Structure (by ref)"))
  (`|ExecutionSequence`
    (:`then_0`
      (`/Engine/EditorBlueprintResources/StandardMacros.DoOnce` false
        (:`Completed`
          (`/Game/Core/Blueprints/FlyingGameState.StartStopwatch` (`self.FlyingGameState`)))))
    (:`then_1`
      (`self.DisableLastGate`)
      (bind _result (`/Engine/EditorBlueprintResources/StandardMacros.IncrementInt` (`self.ActiveGateIndex`))
        (:`  `
          (`KismetSystemLibrary.PrintString` (`KismetStringLibrary.Conv_IntToString` _result))
          (if (>= _result (`KismetArrayLibrary.Array_Length` (`self.Gates`)))
            (set `self.ActiveGateIndex` 0)
            (set `self.bFinalGate` true)
            (elif (`self.bFinalGate`)
              (bind _result_2 (`/Engine/EditorBlueprintResources/StandardMacros.IncrementInt` (`self.LapsCompleted`))
                (:`  `
                  (`/Game/Core/Blueprints/FlyingGameState.LapCompleted` (`self.FlyingGameState`) _result_2)
                  (set `self.bFinalGate` false)))))
          (`self.SetActiveGate`)
          (`self.InitializeNextGate`))))))

(fn `SetActiveGate`
  (returns (Output :type "/Game/Core/Blueprints/Racing_BP/Gate_BP Object Reference"))
  (bind _output_get (set `self.ActiveGateRef` (`|GetArrayItem` (`self.Gates`) (`self.ActiveGateIndex`))))
  (`/Game/Core/Blueprints/Racing_BP/Gate_BP.SetGateActive` _output_get)
  (return _output_get))

(fn `UserConstructionScript`)