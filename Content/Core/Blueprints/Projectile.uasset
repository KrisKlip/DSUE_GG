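; Projectile actor that explodes on first contact and breaks Target actors it strikes.
; Hit, begin-overlap and end-overlap events on its StaticMesh run identical duplicated logic, gated by a Collided flag so only the first fires.
; It spawns an explosion emitter, applies radius damage with impulse to a Target's destructible component, marks it Destroyed, then destroys its own mesh component, leaving the actor itself alive.
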(event `self.StaticMesh.OnComponentHit`
  (params (HitComponent :type "PrimitiveComponent Object Reference") (OtherActor :type "Actor Object Reference") (OtherComp :type "PrimitiveComponent Object Reference") (NormalImpulse :type "Vector Structure") (Hit :type "HitResult Structure (by ref)"))
  (bind _staticmesh (`self.StaticMesh`))
  (if (not (`self.bCollided`))
    (`GameplayStatics.SpawnEmitterAtLocation` "/Game/StarterContent/Particles/P_Explosion.P_Explosion" (`SceneComponent.K2_GetComponentLocation` _staticmesh) (`SceneComponent.K2_GetComponentRotation` _staticmesh) (3.0 3.0 3.0))
    (`KismetSystemLibrary.PrintString` "hIT")
    (bind _astarget (cast `/Game/Core/Blueprints/Target` OtherActor)
      (:`then`
        (`DestructibleComponent.ApplyRadiusDamage` (`/Game/Core/Blueprints/Target.Destructible` _astarget) 10.0 (`SceneComponent.K2_GetComponentLocation` (`self.StaticMesh`)) 500.0 5000.0 true)
        (set `/Game/Core/Blueprints/Target.bDestroyed` true _astarget))
      (:`CastFailed`
        _))
    (`ActorComponent.K2_DestroyComponent` (`self.StaticMesh`))
    (set `self.bCollided` true)))

(event `self.StaticMesh.OnComponentBeginOverlap`
  (params (OverlappedComponent :type "PrimitiveComponent Object Reference") (OtherActor :type "Actor Object Reference") (OtherComp :type "PrimitiveComponent Object Reference") (OtherBodyIndex :type Integer) (bFromSweep :type Boolean) (SweepResult :type "HitResult Structure (by ref)"))
  (bind _staticmesh (`self.StaticMesh`))
  (if (not (`self.bCollided`))
    (`GameplayStatics.SpawnEmitterAtLocation` "/Game/StarterContent/Particles/P_Explosion.P_Explosion" (`SceneComponent.K2_GetComponentLocation` _staticmesh) (`SceneComponent.K2_GetComponentRotation` _staticmesh) (3.0 3.0 3.0))
    (`KismetSystemLibrary.PrintString` "hIT")
    (bind _astarget (cast `/Game/Core/Blueprints/Target` OtherActor)
      (:`then`
        (`DestructibleComponent.ApplyRadiusDamage` (`/Game/Core/Blueprints/Target.Destructible` _astarget) 10.0 (`SceneComponent.K2_GetComponentLocation` (`self.StaticMesh`)) 500.0 5000.0 true)
        (set `/Game/Core/Blueprints/Target.bDestroyed` true _astarget))
      (:`CastFailed`
        _))
    (`ActorComponent.K2_DestroyComponent` (`self.StaticMesh`))
    (set `self.bCollided` true)))

(event `self.StaticMesh.OnComponentEndOverlap`
  (params (OverlappedComponent :type "PrimitiveComponent Object Reference") (OtherActor :type "Actor Object Reference") (OtherComp :type "PrimitiveComponent Object Reference") (OtherBodyIndex :type Integer))
  (bind _staticmesh (`self.StaticMesh`))
  (if (not (`self.bCollided`))
    (`GameplayStatics.SpawnEmitterAtLocation` "/Game/StarterContent/Particles/P_Explosion.P_Explosion" (`SceneComponent.K2_GetComponentLocation` _staticmesh) (`SceneComponent.K2_GetComponentRotation` _staticmesh) (3.0 3.0 3.0))
    (`KismetSystemLibrary.PrintString` "hIT")
    (bind _astarget (cast `/Game/Core/Blueprints/Target` OtherActor)
      (:`then`
        (`DestructibleComponent.ApplyRadiusDamage` (`/Game/Core/Blueprints/Target.Destructible` _astarget) 10.0 (`SceneComponent.K2_GetComponentLocation` (`self.StaticMesh`)) 500.0 5000.0 true)
        (set `/Game/Core/Blueprints/Target.bDestroyed` true _astarget))
      (:`CastFailed`
        _))
    (`ActorComponent.K2_DestroyComponent` (`self.StaticMesh`))
    (set `self.bCollided` true)))

(fn `UserConstructionScript`)