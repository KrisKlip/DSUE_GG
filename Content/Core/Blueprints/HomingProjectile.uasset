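; Homing missile projectile that explodes on its first hit with a radial impulse and particle effect, then destroys itself.
; HomingMissile sets speed and homing strength, seeking a FlyingPawn's HomingLoc or an interface-supplied component, and flies unguided if the target is invalid or destroyed.
; Tick makes all HomingProjectiles ignore each other's collision.
; It also drops homing once the missile overshoots the target's distance from the shooter, destroying it after a delay.
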(event `self.Sphere.OnComponentHit`
  (params (HitComponent :type "PrimitiveComponent Object Reference") (OtherActor :type "Actor Object Reference") (OtherComp :type "PrimitiveComponent Object Reference") (NormalImpulse :type "Vector Structure") (Hit :type "HitResult Structure (by ref)"))
  (bind _explosionforce (`self.ExplosionForce`))
  (`KismetSystemLibrary.PrintString` (`KismetSystemLibrary.GetDisplayName` OtherActor) true true (struct :`R` 0.382369 :`G` 1.0 :`A` 1.0))
  (if (!= OtherActor "HomingProjectile")
    (`/Engine/EditorBlueprintResources/StandardMacros.DoOnce` false
      (:`Completed`
        (`RadialForceComponent.FireImpulse` _explosionforce)
        (`GameplayStatics.SpawnEmitterAtLocation` "/Game/StarterContent/Particles/P_Explosion.P_Explosion" (`SceneComponent.K2_GetComponentLocation` _explosionforce) (struct) (6.0 6.0 6.0))
        (`self.K2_DestroyActor`)
        (`KismetSystemLibrary.PrintString` "Hello")))))

(event `HomingMissile`
  (params (Target :type "Actor Object Reference") (Velocity :type "Float (double-precision)") (Accuracy :type "Float (double-precision)"))
  (bind _projectilemovement (`self.ProjectileMovement`))
  (bind _projectilemovement_2 (`self.ProjectileMovement`))
  (bind _output_get (set `ProjectileMovementComponent.InitialSpeed` Velocity _projectilemovement_2))
  (set `ProjectileMovementComponent.MaxSpeed` (* _output_get 1.333333) _projectilemovement_2)
  (`/Engine/EditorBlueprintResources/StandardMacros.IsValid` Target
    (:`Is Valid`
      (set `self.Target` Target)
      (bind _asflying_pawn (cast `/Game/Core/Blueprints/FlyingPawn` Target)
        (:`then`
          (set `ProjectileMovementComponent.HomingTargetComponent` (`/Game/Core/Blueprints/FlyingPawn.HomingLoc` _asflying_pawn) _projectilemovement)
          (set `ProjectileMovementComponent.HomingAccelerationMagnitude` Accuracy _projectilemovement :!label _label)
          (set `ProjectileMovementComponent.bIsHomingProjectile` true _projectilemovement))
        (:`CastFailed`
          (bind _destroyed (message `/Game/Core/Blueprints/TargetInterface.Destroyed` Target))
          (if _destroyed
            (set `ProjectileMovementComponent.bIsHomingProjectile` false _projectilemovement :!label _label_2)
            (else
              (bind _homingloc (message `/Game/Core/Blueprints/TargetInterface.HomingLocation` Target))
              (set `ProjectileMovementComponent.HomingTargetComponent` _homingloc _projectilemovement)
              (goto _label))))))
    (:`Is Not Valid`
      (goto _label_2))))

(event `self.ReceiveTick`
  (params (DeltaSeconds :type "Float (single-precision)"))
  (bind _sphere (`self.Sphere`))
  (bind _returnvalue (`self.GetDistanceTo` (`self.Shooter`)))
  (bind _returnvalue_2 (+ (`self.GetDistanceTo` (`self.Target`) (`self.Shooter`)) 100.0))
  (bind _outactors (`GameplayStatics.GetAllActorsOfClass` "HomingProjectile_C"))
  (for _array_element _outactors
    (`PrimitiveComponent.IgnoreActorWhenMoving` _sphere _array_element true)
    (`PrimitiveComponent.IgnoreComponentWhenMoving` (`/Game/Core/Blueprints/HomingProjectile.Sphere` _array_element) _sphere true)
    (if (`ProjectileMovementComponent.bIsHomingProjectile` (`self.ProjectileMovement`))
      (`KismetSystemLibrary.PrintString` (`KismetStringLibrary.Conv_DoubleToString` _returnvalue) true true (struct :`R` 0.570318 :`G` 1.0 :`A` 1.0))
      (`KismetSystemLibrary.PrintString` (`KismetStringLibrary.Conv_DoubleToString` _returnvalue_2) true true (struct :`G` 0.14182 :`B` 1.0 :`A` 1.0))
      (if (> _returnvalue _returnvalue_2)
        (set `ProjectileMovementComponent.bIsHomingProjectile` false (`self.ProjectileMovement`))
        (`KismetSystemLibrary.Delay` 2.0)
        (`self.K2_DestroyActor`)))))

(event `self.ReceiveBeginPlay`
  (set `self.StartLocation` (`self.K2_GetActorLocation`)))

(fn `SetShooter`
  (params (Shooter :type "Actor Object Reference"))
  (set `self.Shooter` Shooter))

(fn `UserConstructionScript`)