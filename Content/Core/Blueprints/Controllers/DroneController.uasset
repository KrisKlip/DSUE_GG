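; Player controller that switches possession between FightingPawn and DrawingPawn on keys 1/2, forwarding camera and gate-rotation axes to them.
; Escape or Menu toggles the in-game menu, swapping input mode, reloading saved settings and clearing credits/browser widgets on close.
; Events cover menu creation, listen-server detection, GameInstance registration and session teardown.
; The startup chain calling setup events is disconnected; BeginPlay only caches the FightingPawn.
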(event `Detect Server Type`
  (bind _printdebugonscreen (`self.PrintDebugOnScreen`))
  (bind _printdebugonscreen_2 (`self.PrintDebugOnScreen`))
  ;[1 1 1] Detects if Dedicated Server or Listen Server - Marks Listen Server Player
  (`KismetSystemLibrary.Delay` 1.0)
  (`/Engine/EditorBlueprintResources/ActorMacros.Switch Has Authority`
    (:`Authority`
      (if (`KismetSystemLibrary.IsDedicatedServer`)
        (`KismetSystemLibrary.PrintString` "A Dedicated Server Is Running The Game" _printdebugonscreen _printdebugonscreen)
        (else
          (`|ExecutionSequence`
            (:`then_0`
              (bind _asthird_person_game_state (cast `/Game/ThirdPersonExample/Blueprints/ThirdPersonGameState` (`GameplayStatics.GetGameState`)))
              (if (not (`/Game/ThirdPersonExample/Blueprints/ThirdPersonGameState.IsListenServerAlreadyJoined?` _asthird_person_game_state))
                (set `self.IsListenServer?` true)
                (`KismetSystemLibrary.PrintString` "A Listen Server Is Running The Game" _printdebugonscreen_2 _printdebugonscreen_2)))
            (:`then_1`
              (bind _asthird_person_game_state_2 (cast `/Game/ThirdPersonExample/Blueprints/ThirdPersonGameState` (`GameplayStatics.GetGameState`)))
              (`/Game/ThirdPersonExample/Blueprints/ThirdPersonGameState.Player Join` _asthird_person_game_state_2))))))))

(event `Tell GameInstance The Player Controller`
  ;[1 1 1] Tell GameInstance The Player Controller
  (bind _asbp_game_instance (cast `/Game/Cardinal/MainMenu/Blueprints/BP_GameInstance` (`GameplayStatics.GetGameInstance`)))
  (set `/Game/Cardinal/MainMenu/Blueprints/BP_GameInstance.PlayerController` self _asbp_game_instance))

(event `Hide Mouse`
  (bind _returnvalue (`GameplayStatics.GetPlayerController` 0))
  ;[1 1 1] Hide Mouse
  (`WidgetBlueprintLibrary.SetInputMode_GameOnly` _returnvalue)
  (set `PlayerController.bShowMouseCursor` false _returnvalue))

(event `Load Game Settings`
  ;[1 1 1] Load Game Settings On Controller Creation
  (bind _returnvalue (`GameplayStatics.LoadGameFromSlot` "GameSettings" :!label _label))
  (bind _asbp_game_settings_save (cast `/Game/Cardinal/MainMenu/Blueprints/Saves/BP_GameSettingsSave` _returnvalue))
  (set `self.MouseSensitivity` (`/Game/Cardinal/MainMenu/Blueprints/Saves/BP_GameSettingsSave.MouseSensitivity` _asbp_game_settings_save))
  (set `self.InvertXAxis` (`/Game/Cardinal/MainMenu/Blueprints/Saves/BP_GameSettingsSave.InvertXAxis` _asbp_game_settings_save))
  (set `self.InvertYAxis` (`/Game/Cardinal/MainMenu/Blueprints/Saves/BP_GameSettingsSave.InvertYAxis` _asbp_game_settings_save))
  (set `self.Player FOV` (`/Game/Cardinal/MainMenu/Blueprints/Saves/BP_GameSettingsSave.PlayerFOV` _asbp_game_settings_save))
  (bind _asthird_person_character (cast `/Game/ThirdPersonExample/Blueprints/ThirdPersonCharacter` (`self.K2_GetPawn`)))
  (`CameraComponent.SetFieldOfView` (`/Game/ThirdPersonExample/Blueprints/ThirdPersonCharacter.FollowCamera` _asthird_person_character) (`self.Player FOV`)))

(event `CustomEvent`
  ;[1 1 1] Load Game Settings On Controller Creation
  (goto _label))

(event `CustomEvent_1`
  ;[1 1 1] Load Game Settings On Controller Creation
  (goto _label))

(event `self.ReceiveBeginPlay`
  (`|ExecutionSequence`
    (:`then_0`
      (bind _asfighting_pawn (cast `/Game/Core/Blueprints/Characters/FightingPawn` (`GameplayStatics.GetPlayerPawn` 0)))
      (set `self.CharacterRef` _asfighting_pawn))))

(event `InputAxis|GateRotateForwardBack`
  (params (AxisValue :type "Float (single-precision)"))
  (bind _asdrawing_pawn (cast `/Game/Core/Blueprints/Characters/DrawingPawn` (`self.K2_GetPawn`)))
  (`/Game/Core/Blueprints/Characters/DrawingPawn.PitchActiveGate` _asdrawing_pawn AxisValue))

(event `InputAxis|GateRotateLeftRight`
  (params (AxisValue :type "Float (single-precision)"))
  (bind _asdrawing_pawn (cast `/Game/Core/Blueprints/Characters/DrawingPawn` (`self.K2_GetPawn`)))
  (`/Game/Core/Blueprints/Characters/DrawingPawn.YawACtiveGate` _asdrawing_pawn AxisValue))

(event `Key|Two`
  (params (Key :type "Key Structure"))
  (:`Pressed`
    (bind _outactors (`GameplayStatics.GetAllActorsOfClass` "/Game/Core/Blueprints/Characters/DrawingPawn.DrawingPawn_C"))
    (`self.Possess` (`|GetArrayItem` _outactors))
    (set `/Game/Core/Blueprints/Characters/FightingPawn.bAcceptInput` false (`self.CharacterRef`))))

(event `Key|One`
  (params (Key :type "Key Structure"))
  (:`Pressed`
    (bind _outactors (`GameplayStatics.GetAllActorsOfClass` "/Game/Core/Blueprints/Characters/FightingPawn.FightingPawn_C"))
    (`self.Possess` (`|GetArrayItem` _outactors))
    (set `/Game/Core/Blueprints/Characters/FightingPawn.bAcceptInput` false (`self.CharacterRef`))))

(event `InputAxis|CameraFOV`
  (params (AxisValue :type "Float (single-precision)"))
  (bind _asfighting_pawn (cast `/Game/Core/Blueprints/Characters/FightingPawn` (`self.K2_GetPawn`)))
  (`/Game/Core/Blueprints/Characters/FightingPawn.SetFOV` _asfighting_pawn AxisValue))

(event `InputAxis|CameraAngle`
  (params (AxisValue :type "Float (single-precision)"))
  (bind _asfighting_pawn (cast `/Game/Core/Blueprints/Characters/FightingPawn` (`self.K2_GetPawn`)))
  (`/Game/Core/Blueprints/Characters/FightingPawn.SetCameraAngle` _asfighting_pawn AxisValue))

(event `Create InGameMenu Widget`
  ;[0.08001 1 0.05586] Creates InGameMenu widget
  (bind _returnvalue (`|CreateWidget` "/Game/Cardinal/MainMenu/Blueprints/UI/InGameMenu.InGameMenu_C"))
  (bind _output_get (set `self.InGame Menu` _returnvalue))
  (`UserWidget.AddToViewport` _output_get 5)
  (`Widget.SetVisibility` _output_get "Collapsed")
  (set `/Game/Cardinal/MainMenu/Blueprints/UI/InGameMenu.OwningPlayerController` self _returnvalue)
  (`KismetSystemLibrary.Delay` 2.0)
  (set `/Game/Cardinal/MainMenu/Blueprints/UI/InGameMenu.IsListenServer?` (`self.IsListenServer?`) _returnvalue)
  (`self.Load Game Settings`))

(event `Open Close Game Menu`
  (bind _returnvalue (`GameplayStatics.GetPlayerController` 0))
  (bind _ingame_menu (`self.InGame Menu`))
  (bind _keybindwidget (`/Game/Cardinal/MainMenu/Blueprints/UI/Submenus/SettingsSubMenu.KeyBindWidget` (`/Game/Cardinal/MainMenu/Blueprints/UI/InGameMenu.SettingsSubMenu` (`self.InGame Menu`))))
  ;[0.08001 1 0.05586] Open/close the In Game Menu
  ;;[1 1 0] We avoid to close In Game Menu on rebind open/close menu key. Not the best solution but it works.
  (if (`/Game/Cardinal/MainMenu/Blueprints/UI/SettingsPanels/ControlsSettingsDetails.IsMenuKeyBindPressed` _keybindwidget) :!label _label_2
    (set `/Game/Cardinal/MainMenu/Blueprints/UI/SettingsPanels/ControlsSettingsDetails.IsMenuKeyBindPressed` false _keybindwidget)
    (else
      (`/Engine/EditorBlueprintResources/StandardMacros.FlipFlop`
        (:`A`
          (`Widget.SetVisibility` _ingame_menu "Visible")
          (`WidgetBlueprintLibrary.SetInputMode_GameAndUIEx` _returnvalue null "LockAlways" false)
          (set `PlayerController.bShowMouseCursor` true _returnvalue)
          (`self.SetIgnoreLookInput` _returnvalue true)
          (`VirtualCursorFunctionLibrary.EnableVirtualCursor` _returnvalue))
        (:`B`
          (`Widget.SetVisibility` _ingame_menu "Collapsed")
          (`WidgetBlueprintLibrary.SetInputMode_GameOnly` _returnvalue)
          (set `PlayerController.bShowMouseCursor` false _returnvalue)
          (`VirtualCursorFunctionLibrary.DisableVirtualCursor` _returnvalue)
          (`self.SetIgnoreLookInput` _returnvalue false)
          ;;[1 1 1] Refresh Game Settings From Save On Menu Close
          (`self.Load Game Settings`)
          ;[1 1 1] Remove About Widgets If Open
          (`|ExecutionSequence`
            (:`then_0`
              (bind _foundwidgets (`WidgetBlueprintLibrary.GetAllWidgetsOfClass` "/Game/Cardinal/MainMenu/Blueprints/UI/AboutPanels/Credits.Credits_C"))
              (for _array_element _foundwidgets
                (`Widget.RemoveFromParent` _array_element)))
            (:`then_1`
              (bind _foundwidgets_2 (`WidgetBlueprintLibrary.GetAllWidgetsOfClass` "/Game/Cardinal/MainMenu/Blueprints/UI/AboutPanels/CreditsContainer.CreditsContainer_C"))
              (for _array_element_2 _foundwidgets_2
                (`Widget.RemoveFromParent` _array_element_2)))
            (:`then_2`
              (bind _foundwidgets_3 (`WidgetBlueprintLibrary.GetAllWidgetsOfClass` "/Game/Cardinal/MainMenu/Blueprints/UI/AboutPanels/CreditsNavigation.CreditsNavigation_C"))
              (for _array_element_3 _foundwidgets_3
                (`Widget.RemoveFromParent` _array_element_3)))
            (:`then_3`
              (`|ExecutionSequence`
                (:`then_0`
                  (bind _foundwidgets_4 (`WidgetBlueprintLibrary.GetAllWidgetsOfClass` "/Game/Cardinal/MainMenu/Blueprints/UI/AboutPanels/WebBrowser.WebBrowser_C"))
                  (for _array_element_4 _foundwidgets_4
                    (`Widget.RemoveFromParent` _array_element_4)))
                (:`then_1`
                  (bind _foundwidgets_5 (`WidgetBlueprintLibrary.GetAllWidgetsOfClass` "/Game/Cardinal/MainMenu/Blueprints/UI/AboutPanels/WebBrowserNavigation.WebBrowserNavigation_C"))
                  (for _array_element_5 _foundwidgets_5
                    (`Widget.RemoveFromParent` _array_element_5)))
                (:`then_2`
                  (bind _foundwidgets_6 (`WidgetBlueprintLibrary.GetAllWidgetsOfClass` "/Game/Cardinal/MainMenu/Blueprints/UI/AboutPanels/WebBrowserBackground.WebBrowserBackground_C"))
                  (for _array_element_6 _foundwidgets_6
                    (`Widget.RemoveFromParent` _array_element_6)))
                (:`then_3`
                  (bind _foundwidgets_7 (`WidgetBlueprintLibrary.GetAllWidgetsOfClass` "/Game/Cardinal/MainMenu/Blueprints/UI/AboutPanels/WebBrowserContainer.WebBrowserContainer_C"))
                  (for _array_element_7 _foundwidgets_7
                    (`Widget.RemoveFromParent` _array_element_7)))))))))))

(event `Key|Escape`
  (params (Key :type "Key Structure"))
  ;[0.08001 1 0.05586] Open/close the In Game Menu
  (:`Pressed`
    (goto _label_2)))

(event `Key|Escape`
  (params (Key :type "Key Structure"))
  ;[0.08001 1 0.05586] Open/close the In Game Menu
)

(event `InputAction|Menu`
  (params (Key :type "Key Structure"))
  ;[0.08001 1 0.05586] Open/close the In Game Menu
  (:`Pressed`
    (goto _label_2)))

(event `End Client Online Session`
  (bind _printdebugonscreen (`self.PrintDebugOnScreen`))
  ;[1 1 1] Client End Online Session
  (`DestroySessionCallbackProxy.DestroySession` self
    (:`then`
      (`KismetSystemLibrary.Delay` 1.0)
      (`GameplayStatics.OpenLevel` "MainMenu"))
    (:`OnSuccess`
      (`KismetSystemLibrary.PrintString` "Client Destroy Session Success" _printdebugonscreen _printdebugonscreen))))

(fn `UserConstructionScript`)