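; Game mode for dogfight flying matches that keeps the online session's advertised player count current.
; From BeginPlay, a self-repeating delayed event writes the network player count into the TOTPLAYING extra setting and updates the session, looping on success or failure.
; Player login increments ConnectedPlayers on FlyingGameState and calls its Reset, while logout decrements the count.
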(event `self.ReceiveBeginPlay`
  ;[1 1 1] Update Sessions
  (`self.Update Session`))

(event `Update Session`
  ;[1 1 1] Update Session Settings - Session Properties To Modify
  (`KismetSystemLibrary.Delay` (`self.UpdateSessionsInterval`))
  (`KismetArrayLibrary.Array_Set` (`self.SessionExtraSettings`) 0 (`AdvancedSessionsLibrary.MakeLiteralSessionPropertyString` "TOTPLAYING" (`KismetStringLibrary.Conv_IntToString` (`AdvancedSessionsLibrary.GetNumberOfNetworkPlayers`))) true)
  ;[1 1 1] Update Session
  (bind (_numconnections _numprivateconnections _bislan _bisdedicated _ballowinvites _ballowjoininprogress _bisanticheatenabled _builduniqueid _extrasettings) (`AdvancedSessionsLibrary.GetSessionSettings`)
    (:`OnSuccess`
      (bind _modifiedsettingsarray (`AdvancedSessionsLibrary.AddOrModifyExtraSettings` _extrasettings (`self.SessionExtraSettings`)))
      (`UpdateSessionCallbackProxyAdvanced.UpdateSession` _modifiedsettingsarray _numconnections _numprivateconnections _bislan _ballowinvites _ballowjoininprogress true _bisdedicated
        (:`OnSuccess`
          _)
        (:`OnFailure`
          _)))
    (:`OnFailure`
      _))
  (`self.Update Session`))

(event `self.K2_PostLogin`
  (params (NewPlayer :type "PlayerController Object Reference"))
  (bind _asflying_game_state (cast `/Game/Core/Blueprints/FlyingGameState` (`GameplayStatics.GetGameState`)))
  (`/Engine/EditorBlueprintResources/StandardMacros.IncrementInt` (`/Game/Core/Blueprints/FlyingGameState.ConnectedPlayers` _asflying_game_state)
    (:`  `
      (`/Game/Core/Blueprints/FlyingGameState.Reset` _asflying_game_state))))

(event `self.K2_OnLogout`
  (params (ExitingController :type "Controller Object Reference"))
  (bind _asflying_game_state (cast `/Game/Core/Blueprints/FlyingGameState` (`GameplayStatics.GetGameState`)))
  (`/Engine/EditorBlueprintResources/StandardMacros.DecrementInt` (`/Game/Core/Blueprints/FlyingGameState.ConnectedPlayers` _asflying_game_state)))

(fn `UserConstructionScript`)